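; BP_Door is a networked swinging door that toggles open and closed through the Serv_Door event.
; The event flips Open and plays or reverses a timeline that yaws the root component up to 90 degrees in the negative direction.
; An OnRep function for Open reapplies the stored RotationZ to the root.
; The box overlap checks for BP_ThirdPersonCharacter but takes no action.
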(event `Serv_Door`
  (if (not (`self.Open?`))
    (set `self.Open?` true)
    (bind (_direction _rotationz_) (`Timeline|OpenCloseTimeline` :!label _label)
      (:`Update`
        (bind _output_get (set `self.Rotation Z` (* _rotationz_ -90.0)))
        (`SceneComponent.K2_SetRelativeRotation` (`self.DefaultSceneRoot`) (`KismetMathLibrary.MakeRotator` 0.0 0.0 _output_get) false false)))
    (else
      (set `self.Open?` false)
      (goto _label :!via `Reverse`))))

(event `self.Box.OnComponentBeginOverlap`
  (params (OverlappedComponent :type "PrimitiveComponent Object Reference") (OtherActor :type "Actor Object Reference") (OtherComp :type "PrimitiveComponent Object Reference") (OtherBodyIndex :type Integer) (bFromSweep :type Boolean) (SweepResult :type "HitResult Structure (by ref)"))
  (if (== OtherActor "/Game/ThirdPerson/Blueprints/BP_ThirdPersonCharacter.BP_ThirdPersonCharacter")
    _))

(fn `OnRep_Open?`
  (`SceneComponent.K2_SetRelativeRotation` (`self.DefaultSceneRoot`) (`KismetMathLibrary.MakeRotator` 0.0 0.0 (`self.Rotation Z`)) false false))

(fn `UserConstructionScript`)